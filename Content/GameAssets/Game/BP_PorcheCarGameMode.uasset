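; Game mode for the Porche car game that runs a countdown to a loss, extended by crossing checkpoints.
; BeginPlay starts a short one-shot timer bound to YouLose and shows the time-check widget.
; CheckPointCrossed re-sets that timer to its remaining time plus a fixed bonus.
; YouLose shows the lose screen on expiry, while YouWon only clears the timer and logs it.
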(event Custom|YouLose
  (bind _returnvalue (UserInterface|CreateWidget "/Game/GameAssets/Game/Widgets/UI_YouLose.UI_YouLose_C"))
  (UserInterface|Viewport|AddtoViewport _returnvalue 0))

(event Custom|YouWon
  (Utilities|Time|ClearandInvalidateTimerbyHandle (Variables|Default|GetTimeRemainingTimerHandle))
  (Development|PrintString "Log : Timer Invalidated"))

(event Custom|Check%20Point%20Crossed
  (bind _returnvalue (Utilities|Time|SetTimerbyEvent (delegate Custom|YouLose) (+ (Utilities|Time|GetTimerRemainingTimebyHandle (Variables|Default|GetTimeRemainingTimerHandle)) 5e+01)))
  (Variables|Default|SetTimeRemainingTimerHandle _returnvalue))

(event EventBeginPlay
  (bind _returnvalue (Utilities|Time|SetTimerbyEvent (delegate Custom|YouLose) 5.0))
  (Variables|Default|SetTimeRemainingTimerHandle _returnvalue)
  (bind _returnvalue_2 (UserInterface|CreateWidget "/Game/GameAssets/Game/Widgets/UI_TimeCheck.UI_TimeCheck_C"))
  (UserInterface|Viewport|AddtoViewport _returnvalue_2 0))

(event EventTick
  (params (DeltaSeconds :type Float%20%28single-precision%29)))

(fn ConstructionScript)